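; Toy dispenser cannon Blueprint that keeps its base aimed at a targeting reticle.
; Every tick it rotates CannonBase in world space to look at the root of the TargetRetical child actor.
; BeginPlay and construction only call the parent class, so this graph adds just the aiming behavior.
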(event `self.ReceiveBeginPlay`
  (`parent.ReceiveBeginPlay`))

(event `self.ReceiveTick`
  (params (DeltaSeconds :type "Float (single-precision)"))
  (`SceneComponent.K2_SetWorldRotation` (`self.CannonBase`) (`KismetMathLibrary.FindLookAtRotation` (`SceneComponent.K2_GetComponentLocation` (`self.CannonBase`)) (`SceneComponent.K2_GetComponentLocation` (`Actor.RootComponent` (`ChildActorComponent.ChildActor` (`self.Target Retical`))))) false false))

(fn `UserConstructionScript`
  (`parent.UserConstructionScript`))