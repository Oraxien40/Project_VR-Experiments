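; BP_StatChanger is a toy actor with a Board component and a return button that brings the board back to its starting spot.
; On BeginPlay it records the Board's relative location as its origin.
; When a VRPawn overlaps the button's collision box, it reattaches the Board to the root, keeping world position and rotation, then moves it back to that origin with MoveComponentTo.
; No stat-changing logic appears in its graphs.
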(event `self.ReceiveBeginPlay`
  ;[1 1 1] Set Board Origin
  (set `self.Board Origin` (`SceneComponent.RelativeLocation` (`self.Board`))))

(event `self.ReturnButtonCollisionBox.OnComponentBeginOverlap`
  (params (OverlappedComponent :type "PrimitiveComponent Object Reference") (OtherActor :type "Actor Object Reference") (OtherComp :type "PrimitiveComponent Object Reference") (OtherBodyIndex :type Integer) (bFromSweep :type Boolean) (SweepResult :type "HitResult Structure (by ref)"))
  (cast `/Game/VRTemplate/Blueprints/VRPawn` OtherActor)
  (`SceneComponent.K2_AttachToComponent` (`self.Board`) (`self.DefaultSceneRoot`) "None" "KeepWorld" "KeepWorld" "KeepRelative" true)
  (`KismetSystemLibrary.MoveComponentTo` (`self.Board`) (`self.Board Origin`)))

(fn `UserConstructionScript`)